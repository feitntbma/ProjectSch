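; BP_Door is a clickable door in the school level's start area, tagged with a difficulty of Easy, Hard or Impossible.
; It enables mouse click events on BeginPlay and reacts to clicks on its static mesh.
; Depending on GameState, a click either opens Widget_Info with the door's difficulty and switches to UI-only input, or restores game-and-UI input.
; The switch on difficulty itself has empty branches.
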(event OnClicked(StaticMesh)
  (params (TouchedComponent :type Primitive%20Component%20Object%20Reference) (ButtonPressed :type Key%20Structure :default "None"))
  (bind _returnvalue (Game|GetPlayerController 0))
  (bind _levelofdoor (Variables|Default|Getlevelofdoor))
  (switch Utilities|FlowControl|Switch|SwitchonEnum_States _levelofdoor
    (:NewEnumerator0
      _)
    (:NewEnumerator1
      _)
    (:NewEnumerator2
      _))
  (switch Utilities|FlowControl|Switch|SwitchonEnum_GameState (Variables|Default|Getgame_state)
    (:NewEnumerator0
      (bind _returnvalue_2 (UserInterface|CreateWidget "/Game/LevelSchool/Start/BP/WidgetBP/Widget_Info.Widget_Info_C" 0 0 _levelofdoor))
      (bind _output_get (Variables|Default|Seta _returnvalue_2))
      (UserInterface|Viewport|AddtoViewport _output_get 0)
      (Input|SetInputModeUIOnly _returnvalue _output_get "DoNotLock"))
    (:NewEnumerator1
      (Input|SetInputModeGameandUI _returnvalue 0 "DoNotLock" false))))

(event EventBeginPlay
  (Variables|/Script/Engine.PlayerController|SetbEnableClickEvents (Game|GetPlayerController 0) true))

(event Collision|EventActorBeginOverlap
  (params (OtherActor :type Actor%20Object%20Reference)))

(event EventTick
  (params (DeltaSeconds :type Float%20%28single-precision%29)))

(fn ConstructionScript)