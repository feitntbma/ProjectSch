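; BP_SCORE is an actor Blueprint that keeps a score counter and a Lvl counter for the school level.
; ADD raises POINTS by one and SUBSTR lowers it by one, while both increment Lvl, so Lvl counts every scoring call regardless of result.
; Print shows the current POINTS as a debug string, and the event graph and construction script contain no logic.
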(event EventBeginPlay)

(event Collision|EventActorBeginOverlap
  (params (OtherActor :type Actor%20Object%20Reference)))

(event EventTick
  (params (DeltaSeconds :type Float%20%28single-precision%29)))

(fn ConstructionScript)

(fn ADD
  (Variables|Default|SetPOINTS (+ (Variables|Default|GetPOINTS) 1))
  (Variables|Default|SetLvl (+ 1 (Variables|Default|GetLvl))))

(fn SUBSTR
  (Variables|Default|SetPOINTS (- (Variables|Default|GetPOINTS) 1))
  (Variables|Default|SetLvl (+ 1 (Variables|Default|GetLvl))))

(fn Print
  (Development|PrintString (Utilities|String|ToString(Integer) (Variables|Default|GetPOINTS))))